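; Player HUD Blueprint that shows the in-game UI and switches to a win or lose menu when the match ends.
; BeginPlay sets game-only input and normal time, pre-creates the three widgets and displays the main UI.
; Tick polls a WinConditionManager, supplied through SetWCManager, for GameWon or GameLost.
; Either result swaps widgets, enables UI-only input and cursor, and freezes time via global dilation, with no one-shot guard.
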(event `self.ReceiveBeginPlay`
  (bind _returnvalue (`GameplayStatics.GetPlayerController` 0))
  (set `PlayerController.bShowMouseCursor` false _returnvalue)
  (`WidgetBlueprintLibrary.SetInputMode_GameOnly` _returnvalue true)
  (`GameplayStatics.SetGlobalTimeDilation` 1.0)
  (bind _returnvalue_2 (`|CreateWidget` "/Game/GameContent/WB_WinMenu.WB_WinMenu_C"))
  (set `self.WinMenu` _returnvalue_2)
  (bind _returnvalue_3 (`|CreateWidget` "/Game/GameContent/WB_LoseMenu.WB_LoseMenu_C"))
  (set `self.LoseMenu` _returnvalue_3)
  (bind _returnvalue_4 (`|CreateWidget` "/Game/GameContent/WB_IngameUI.WB_IngameUI_C"))
  (set `self.MainUI` _returnvalue_4)
  (`UserWidget.AddToViewport` (`self.MainUI`) 0))

(event `self.ReceiveTick`
  (params (DeltaSeconds :type "Float (single-precision)"))
  (bind _returnvalue (`GameplayStatics.GetPlayerController` 0))
  (`/Engine/EditorBlueprintResources/StandardMacros.IsValid` (`self.WinConditionManager`)
    (:`Is Valid`
      (if (`WinConditionManager.bGameWon` (`self.WinConditionManager`))
        (`Widget.RemoveFromParent` (`self.MainUI`))
        (`UserWidget.AddToViewport` (`self.WinMenu`) 0)
        (`WidgetBlueprintLibrary.SetInputMode_UIOnlyEx` _returnvalue null :!label _label)
        (set `PlayerController.bShowMouseCursor` true _returnvalue)
        (`GameplayStatics.SetGlobalTimeDilation` 0.0)
        (elif (`WinConditionManager.bGameLost` (`self.WinConditionManager`))
          (`Widget.RemoveFromParent` (`self.MainUI`))
          (`UserWidget.AddToViewport` (`self.LoseMenu`) 0)
          (goto _label))))))

(fn `SetWCManager`
  (params (WCManage :type "/Game/GameContent/BP_WinConditionManager Object Reference"))
  (set `self.WinConditionManager` WCManage))

(fn `UserConstructionScript`)